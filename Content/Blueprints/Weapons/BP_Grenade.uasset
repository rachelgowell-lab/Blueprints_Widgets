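; Grenade weapon actor that is launched as a projectile and explodes on impact.
; Ignite detaches it from its parent, adds a projectile movement component at runtime with velocity along the fire direction, and enables mesh collision.
; A mesh hit on anything but the owner spawns an emitter, applies radial damage with falloff, and destroys the actor.
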(event OnComponentHit(SM_grenade)
  (params (HitComponent :type Primitive%20Component%20Object%20Reference) (OtherActor :type Actor%20Object%20Reference) (OtherComp :type Primitive%20Component%20Object%20Reference) (NormalImpulse :type Vector :default "0, 0, 0") (Hit :type Hit%20Result%20Structure%20%28by%20ref%29))
  (if (!= OtherActor (Components|GetOwner))
    (Effects|SpawnEmitteratLocation 0 (Transformation|GetActorLocation))
    (Class|GameplayStatics|ApplyRadialDamagewithFalloff (Variables|Default|GetBase%20Damage) 0.0 (Transformation|GetActorLocation) 0.0 (Variables|Default|GetDamage%20Outer%20Radius) 1.0 0 0 self 0 "ECC_Visibility")
    (Actor|DestroyActor)))

(event Custom|Ignite
  (params (FireDirection :type Vector))
  ;[0.15 0.15 0.15 0.5] Ignite
  (Transformation|DetachFromActor "KeepWorld" "KeepWorld" "KeepWorld")
  (bind _returnvalue (AddComponent|AddProjectileMovementComponent))
  (Variables|/Script/Engine.MovementComponent|SetVelocity _returnvalue (* FireDirection (Variables|Default|GetProjectile%20Speed)))
  (Collision|SetCollisionEnabled (Variables|Default|GetSM_grenade) "QueryAndPhysics"))

(event EventBeginPlay
  (|CallParentFunction) ; This node is disabled and will not be called.\nDrag off pins to build functionality.
)

(event Collision|EventActorBeginOverlap
  (params (OtherActor :type Actor%20Object%20Reference))
  (|CallParentFunction OtherActor) ; This node is disabled and will not be called.\nDrag off pins to build functionality.
)

(event EventTick
  (params (DeltaSeconds :type Float%20%28single-precision%29))
  (|CallParentFunction DeltaSeconds) ; This node is disabled and will not be called.\nDrag off pins to build functionality.
)

(fn ConstructionScript
  (|CallParentFunction))