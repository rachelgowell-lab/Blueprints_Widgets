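; Base character Blueprint that handles weapon acquisition and exposes weapon-specific animations.
; AcquireNewWeapon spawns the given class at the mesh socket named by its class defaults and snap-attaches it there, but sets CurrentActiveWeapon to None rather than the spawned actor.
; GetActveWeapomAnims returns idle and walk animations from CurrentActiveWeapon.
; SwitchActiveWeaponTo only calls PlayMontage on the mesh, with no montage specified.
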(event Custom|AcquireNewWeapon
  (params (WeaponClass :type BP%20Weapon%20Base%20Class%20Reference))
  (bind _equipsocketname (Utilities|GetClassDefaults WeaponClass))
  (bind _self self)
  (Variables|Default|SetCurrentActiveWeapon 0)
  (bind _returnvalue (Game|SpawnActorfromClass WeaponClass (Transformation|GetSocketTransform (Variables|Character|GetMesh) _equipsocketname "RTS_World") "Undefined" "MultiplyWithRoot" _self _self))
  (Variables|Default|SetCurrentActiveWeapon 0)
  (Transformation|AttachComponentToComponent _returnvalue (Variables|Character|GetMesh) _equipsocketname "SnapToTarget" "SnapToTarget" "SnapToTarget" true))

(event Custom|SwitchActiveWeaponTo
  (Animation|Montage|PlayMontage (Variables|Character|GetMesh) 0))

(event EventBeginPlay)

(event Collision|EventActorBeginOverlap
  (params (OtherActor :type Actor%20Object%20Reference)))

(event EventTick
  (params (DeltaSeconds :type Float%20%28single-precision%29)))

(fn ConstructionScript)

(fn GetActveWeapomAnims
  (bind _currentactiveweapon (Variables|Default|GetCurrentActiveWeapon))
  (return (Variables|/Game/Blueprints/Weapons/BP_WeaponBase.BP_WeaponBase_C|GetIdleAnim _currentactiveweapon) (Variables|/Game/Blueprints/Weapons/BP_WeaponBase.BP_WeaponBase_C|GetWalkAnim _currentactiveweapon)))